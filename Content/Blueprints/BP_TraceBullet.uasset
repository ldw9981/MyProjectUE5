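; BP_TraceBullet is a homing projectile that damages the actor it hits.
; While the target passed to SetTarget is valid, Tick faces it and sets projectile velocity to the unnormalized offset, so speed scales with distance.
; On sphere hit it applies fixed damage, reports a "Bullet"-tagged damage event to AI perception using the location saved at BeginPlay as origin, then destroys itself.
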(event `self.ReceiveBeginPlay`
  (set `self.NewVar` (`self.K2_GetActorLocation`)))

(event `self.ReceiveTick`
  (params (DeltaSeconds :type "Float (single-precision)"))
  (bind _returnvalue (`self.K2_GetActorLocation`))
  (bind _returnvalue_2 (`self.K2_GetActorLocation` (`self.Target`)))
  (`/Engine/EditorBlueprintResources/StandardMacros.IsValid` (`self.Target`)
    (:`Is Valid`
      (`self.K2_SetActorRotation` (`KismetMathLibrary.FindLookAtRotation` _returnvalue _returnvalue_2))
      (set `MovementComponent.Velocity` (- _returnvalue_2 _returnvalue) (`self.ProjectileMovement`)))))

(event `self.Sphere.OnComponentHit`
  (params (HitComponent :type "PrimitiveComponent Object Reference") (OtherActor :type "Actor Object Reference") (OtherComp :type "PrimitiveComponent Object Reference") (NormalImpulse :type "Vector Structure") (Hit :type "HitResult Structure (by ref)"))
  (bind _returnvalue (`self.GetInstigatorController`))
  (bind _returnvalue_2 (`GameplayStatics.ApplyDamage` OtherActor 30.0 _returnvalue self))
  (`AISense_Damage.ReportDamageEvent` OtherActor _returnvalue _returnvalue_2 (`self.NewVar`) (`.Location` (`GameplayStatics.BreakHitResult` Hit)) "Bullet")
  (`self.K2_DestroyActor`))

(event `/Game/Blueprints/BPI_Target.SetTarget`
  (params (Actor :type "Actor Object Reference"))
  (set `self.Target` Actor))

(fn `UserConstructionScript`)