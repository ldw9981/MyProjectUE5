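; Zombie enemy whose name, level and combat stats are loaded from DT_MonsterInfo by MonsterID in the construction script.
; BeginPlay binds its health widget to the ability stat component and runs the BT_MonsterRandomPatrol behavior tree.
; Health changes write HealthPercent to the Blackboard while alive.
; At zero health it grants the player table-defined exp, gold and score, disables capsule collision, stops AI logic and destroys itself after a delay.
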(event `self.ReceiveBeginPlay`
  (`|ExecutionSequence`
    (:`then_0`
      (bind _aswbp_health (cast `/Game/Blueprints/Widget/WBP_Health` (`WidgetComponent.GetUserWidgetObject` (`self.Widget`))))
      (set `/Game/Blueprints/Widget/WBP_Health.AbilityStat` (`self.BP_AbilityStat`) _aswbp_health)
      (set `/Game/Blueprints/Widget/WBP_Health.OwnerActor` self _aswbp_health))
    (:`then_1`
      (`AIController.RunBehaviorTree` (`AIBlueprintHelperLibrary.GetAIController` self) "/Game/Blueprints/AI/BT_MonsterRandomPatrol.BT_MonsterRandomPatrol"))))

(event `self.ReceiveActorBeginOverlap`
  (params (OtherActor :type "Actor Object Reference")))

(event `self.BP_AbilityStat.OnChangeHealth`
  (params (Prev :type "Float (double-precision)") (Curr :type "Float (double-precision)"))
  (if (<= Curr 0.0)
    (`|ExecutionSequence`
      (:`then_0`
        (bind _asbp_my_player_character (cast `/Game/Blueprints/BP_MyPlayerCharacter` (`GameplayStatics.GetPlayerCharacter` 0)))
        (bind _returnvalue (`|GetDataTableRow` "/Game/Blueprints/Data/DT_MonsterInfo.DT_MonsterInfo" (`self.MonsterID`))
          (:`then`
            (bind (_name _level _health _attack _defense _rewardgold _rewardexp _rewardscore) (break `/Game/Blueprints/FMonsterInfo` _returnvalue))
            (`/Game/Blueprints/BP_MyPlayerCharacter.GetReward` _asbp_my_player_character _rewardexp _rewardgold _rewardscore))))
      (:`then_1`
        (`PrimitiveComponent.SetCollisionEnabled` (`self.CapsuleComponent`) "NoCollision")
        (`BrainComponent.StopLogic` (`AIController.BrainComponent` (`AIBlueprintHelperLibrary.GetAIController` self)) "Death"))
      (:`then_2`
        (`KismetSystemLibrary.Delay` 3.0)
        (`self.K2_DestroyActor`)))
    (else
      ;[1 1 1] 현재 HealthPercent를 블랙보드에 기록
      (bind _percent (`/Game/Blueprints/BP_AbilityStat.GetHealthPercent` (`self.BP_AbilityStat`)))
      (`BlackboardComponent.SetValueAsFloat` (`AIController.Blackboard` (`AIBlueprintHelperLibrary.GetAIController` self)) "HealthPercent" _percent))))

(fn `UserConstructionScript`
  (bind _bp_abilitystat (`self.BP_AbilityStat`))
  ;[1 1 1] 블루프린트를 수정하거나 게임을 시작할때 BeginPlay이전에 호출함
  (bind _returnvalue (`|GetDataTableRow` "/Game/Blueprints/Data/DT_MonsterInfo.DT_MonsterInfo" (`self.MonsterID`))
    (:`then`
      (bind (_name _level _health _attack _defense) (break `/Game/Blueprints/FMonsterInfo` _returnvalue))
      (set `/Game/Blueprints/BP_AbilityStat.Name` _name _bp_abilitystat)
      (set `/Game/Blueprints/BP_AbilityStat.InitialMaxHealth` _health _bp_abilitystat)
      (set `/Game/Blueprints/BP_AbilityStat.InitialAttack` _attack _bp_abilitystat)
      (set `/Game/Blueprints/BP_AbilityStat.InitialDefense` _defense _bp_abilitystat)
      (set `/Game/Blueprints/BP_AbilityStat.Level` _level _bp_abilitystat))))