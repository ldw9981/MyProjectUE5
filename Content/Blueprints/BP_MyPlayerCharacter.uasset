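; Player character for a shooter, with Enhanced Input movement, a HUD, gun and chargeable grenade.
; Firing traces from screen center to aim bullets from the muzzle, adding timeline recoil, sound and flash.
; Grenade hold time drives launch speed through a curve.
; Radial damage knocks the character back, zero health destroys it after a delay, and GetReward loops level-ups against an experience DataTable.
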(event `self.ReceiveDestroyed`
  (`Widget.RemoveFromParent` (`self.HUD`)))

(event `self.ReceiveBeginPlay`
  (`|ExecutionSequence`
    (:`then_0`
      (bind _returnvalue (`|CreateWidget` "/Game/Blueprints/Widget/WBP_PlayerHUD.WBP_PlayerHUD_C" (`GameplayStatics.GetPlayerController` 0)))
      (set `self.HUD` _returnvalue)
      (set `/Game/Blueprints/Widget/WBP_PlayerHUD.AbilityStat` (`self.BP_AbilityStat`) _returnvalue)
      (set `/Game/Blueprints/Widget/WBP_PlayerHUD.MyPlayerCharacter` self _returnvalue)
      (`UserWidget.AddToViewport` _returnvalue 0))
    (:`then_1`
      (`EnhancedInputSubsystemInterface.AddMappingContext` (pcsubsystem `EnhancedInputLocalPlayerSubsystem` (`GameplayStatics.GetPlayerController` 0)) "/Game/Input/IMC_MyDefault.IMC_MyDefault" 0 (struct)))))

(event `EnhancedInput|/Game/Input/IA_MyLook`
  (params (ActionValue :type "Vector2D Structure") (ElapsedSeconds :type "Float (double-precision)") (TriggeredSeconds :type "Float (double-precision)") (InputAction :type "InputAction Object Reference" :default "/Game/Input/IA_MyLook.IA_MyLook"))
  (bind (_x _y) (`KismetMathLibrary.BreakVector2D` ActionValue))
  (:`Triggered`
    (`self.AddControllerYawInput` _x)
    (`self.AddControllerPitchInput` _y)))

(event `EnhancedInput|/Game/Input/IA_MyMove`
  (params (ActionValue :type "Vector2D Structure") (ElapsedSeconds :type "Float (double-precision)") (TriggeredSeconds :type "Float (double-precision)") (InputAction :type "InputAction Object Reference" :default "/Game/Input/IA_MyMove.IA_MyMove"))
  (bind _returnvalue (`self.GetControlRotation`))
  (bind (_x _y) (`KismetMathLibrary.BreakVector2D` ActionValue))
  (:`Triggered`
    (`self.AddMovementInput` (`KismetMathLibrary.GetRightVector` _returnvalue) _x)
    (`self.AddMovementInput` (`KismetMathLibrary.GetForwardVector` _returnvalue) _y)))

(event `EnhancedInput|/Game/Input/IA_MyJump`
  (params (ActionValue :type Boolean) (ElapsedSeconds :type "Float (double-precision)") (TriggeredSeconds :type "Float (double-precision)") (InputAction :type "InputAction Object Reference" :default "/Game/Input/IA_MyJump.IA_MyJump"))
  (:`Started`
    (`self.Jump`)))

(event `self.ReceiveTick`
  (params (DeltaSeconds :type "Float (single-precision)"))
  (`|ExecutionSequence`
    (:`then_0`
      (if (`KismetMathLibrary.Vector_IsZero` (`self.GetLastMovementInputVector`))
        (set `CharacterMovementComponent.bUseControllerDesiredRotation` false (`self.CharacterMovement`))
        (else
          (set `CharacterMovementComponent.bUseControllerDesiredRotation` true (`self.CharacterMovement`)))))
    (:`then_1`
      (`SceneComponent.K2_SetWorldRotation` (`self.ArrowGrenade`) (`self.GetControlRotation`) false false))))

(event `EnhancedInput|/Game/Input/IA_MyFire`
  (params (ActionValue :type Boolean) (ElapsedSeconds :type "Float (double-precision)") (TriggeredSeconds :type "Float (double-precision)") (InputAction :type "InputAction Object Reference" :default "/Game/Input/IA_MyFire.IA_MyFire"))
  (:`Triggered`
    (`KismetSystemLibrary.Delay` 0.1)
    (if (> (`self.LoadedBullet`) 0)
      (bind _spawn (`self.GetBulletSpawnTransform`))
      (`|SpawnActorFromClass` "/Game/Blueprints/BP_Bullet.BP_Bullet_C" _spawn "Undefined" "OverrideRootScale" null 20.0 self)
      (`|ExecutionSequence`
        (:`then_0`
          (set `self.Recoil` 0.0)
          (bind (_direction _recoil) (`Timeline|타임라인` :!via `PlayFromStart`)
            (:`Update`
              (`self.AddControllerPitchInput` (- (`self.Recoil`) _recoil))
              (set `self.Recoil` _recoil))))
        (:`then_1`
          (bind _location (.location _spawn))
          (`GameplayStatics.PlaySoundAtLocation` "/Game/Blueprints/Sound/SC_Fire.SC_Fire" _location (struct) 1.0 1.0 0.0 null null null null)
          (`GameplayStatics.SpawnEmitterAttached` "/Game/BallisticsVFX/Particles/Muzzle/MuzzleFlash/Muzzle_Flash_Med.Muzzle_Flash_Med" (`self.SkeletalMesh`) "Muzzle" _location (.rotation _spawn) (1.0 1.0 1.0) "KeepWorldPosition"))))))

(event `self.BP_AbilityStat.OnChangeHealth`
  (params (Prev :type "Float (double-precision)") (Curr :type "Float (double-precision)"))
  (if (<= Curr 0.0)
    (`KismetSystemLibrary.Delay` 3.0)
    (`self.K2_DestroyActor`)))

(event `EnhancedInput|/Game/Input/IA_MyGrenade`
  (params (ActionValue :type Boolean) (ElapsedSeconds :type "Float (double-precision)") (TriggeredSeconds :type "Float (double-precision)") (InputAction :type "InputAction Object Reference" :default "/Game/Input/IA_MyGrenade.IA_MyGrenade"))
  (bind _returnvalue (`CurveFloat.GetFloatValue` (`self.GrenadeCharge`) (- (`KismetSystemLibrary.GetGameTimeInSeconds`) (`self.ThowTime`))))
  (:`Started`
    (set `self.ThowTime` (`KismetSystemLibrary.GetGameTimeInSeconds`)))
  (:`Completed`
    (`|SpawnActorFromClass` "/Game/Blueprints/BP_Grenade.BP_Grenade_C" (`SceneComponent.K2_GetComponentToWorld` (`self.ArrowGrenade`)) "Undefined" "OverrideRootScale" null _returnvalue _returnvalue 30.0 self)))

(event `Key|One`
  (params (Key :type "Key Structure")))

(event `self.ReceiveRadialDamage`
  (params (DamageReceived :type "Float (single-precision)") (DamageType :type "DamageType Object Reference") (Origin :type "Vector Structure") (HitInfo :type "HitResult Structure (by ref)") (InstigatedBy :type "Controller Object Reference") (DamageCauser :type "Actor Object Reference"))
  ;[1 1 1] 좀비 속도0 변경
  (`MovementComponent.StopMovementImmediately` (`self.CharacterMovement`))
  (`CharacterMovementComponent.AddImpulse` (`self.CharacterMovement`) (* (`KismetMathLibrary.GetDirectionUnitVector` (`self.K2_GetActorLocation` DamageCauser) (`self.K2_GetActorLocation`)) (`self.Impulse`)) false))

(fn `AddLoadedBullet`
  (params (Value :type Integer)))

(fn `GetBulletSpawnTransform`
  (returns (Spawn :type "Transform Structure"))
  (locals (End :type "Vector Structure" :default (0.0 0.0 0.0)))
  (bind (_x _y) (`KismetMathLibrary.BreakVector2D` (`WidgetLayoutLibrary.GetViewportSize`)))
  (bind _returnvalue (`SceneComponent.GetSocketLocation` (`self.SkeletalMesh`) "Muzzle"))
  (bind (_worldposition _worlddirection) (`GameplayStatics.DeprojectScreenToWorld` (`GameplayStatics.GetPlayerController` 0) (`KismetMathLibrary.MakeVector2D` (/ _x 2.0) (/ _y 2.0))))
  (`KismetSystemLibrary.PrintString` (`KismetStringLibrary.Concat_StrStr` "HELLO:" (`KismetStringLibrary.Conv_IntToString` (`self.Exp`))))
  (bind (_outhit _returnvalue_2) (`KismetSystemLibrary.LineTraceSingle` _worldposition (+ _worldposition (* _worlddirection (100000.0 100000.0 100000.0))) "TraceTypeQuery3"))
  (if _returnvalue_2
    (bind (_bblockinghit _binitialoverlap _time _distance _location _impactpoint _normal _impactnormal _physmat _hitactor _hitcomponent _hitbonename _bonename _hititem _elementindex _faceindex _tracestart _traceend) (`GameplayStatics.BreakHitResult` _outhit))
    (set `local.End` _impactpoint)
    (else
      (set `local.End` _traceend)))
  (return (`KismetMathLibrary.MakeTransform` _returnvalue (`KismetMathLibrary.FindLookAtRotation` _returnvalue (`local.End`)))))

(fn `GetReward`
  (params (Exp :type Integer) (Gold :type Integer) (Score :type Integer))
  (bind _bp_abilitystat (`self.BP_AbilityStat`))
  (set `self.Exp` (+ (`self.Exp`) Exp))
  (bind _returnvalue (`|GetDataTableRow` "/Game/Blueprints/Data/DT_LevelUpExp.DT_LevelUpExp" (`KismetStringLibrary.Conv_StringToName` (`KismetStringLibrary.Conv_IntToString` (`/Game/Blueprints/BP_AbilityStat.Level` (`self.BP_AbilityStat`)))) :!label _label)
    (:`then`
      (bind _exp (break `/Game/Blueprints/FLevelUpExp` _returnvalue))
      (if (>= (`self.Exp`) _exp)
        (set `self.Exp` (- (`self.Exp`) _exp))
        (set `/Game/Blueprints/BP_AbilityStat.Level` (+ (`/Game/Blueprints/BP_AbilityStat.Level` _bp_abilitystat) 1) _bp_abilitystat)
        (goto _label)))))

(fn `UserConstructionScript`)