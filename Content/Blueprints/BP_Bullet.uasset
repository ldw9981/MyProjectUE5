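; Bullet actor that damages whatever its collision sphere hits, tripling damage on a "Head" bone hit, then destroys itself.
; Reports each hit as a damage event, passing the location saved at BeginPlay as the event origin.
; Looks up the hit's physical surface type in DT_BulletEffect to play a sound and attach a reflection-aligned particle and short-lived decal to the hit component.
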(event `self.ReceiveBeginPlay`
  (set `self.NewVar` (`self.K2_GetActorLocation`)))

(event `self.Sphere.OnComponentHit`
  (params (HitComponent :type "PrimitiveComponent Object Reference") (OtherActor :type "Actor Object Reference") (OtherComp :type "PrimitiveComponent Object Reference") (NormalImpulse :type "Vector Structure") (Hit :type "HitResult Structure (by ref)"))
  (bind _returnvalue (`self.GetInstigatorController`))
  (bind (_bblockinghit _binitialoverlap _time _distance _location _impactpoint _normal _impactnormal _physmat _hitactor _hitcomponent _hitbonename _bonename _hititem _elementindex _faceindex _tracestart _traceend) (`GameplayStatics.BreakHitResult` Hit))
  (bind _returnvalue_2 (`GameplayStatics.ApplyDamage` OtherActor (* (`self.Base Damage`) (`KismetMathLibrary.SelectFloat` 3.0 1.0 (== _hitbonename "Head"))) _returnvalue self))
  (`AISense_Damage.ReportDamageEvent` OtherActor _returnvalue _returnvalue_2 (`self.NewVar`) _location)
  (`|ExecutionSequence`
    (:`then_0`
      (`/Engine/EditorBlueprintResources/StandardMacros.IsValid` _physmat
        (:`Is Valid`
          (bind _returnvalue_3 (`|GetDataTableRow` "/Game/Blueprints/Data/DT_BulletEffect.DT_BulletEffect" (`KismetStringLibrary.Conv_StringToName` (`|GetEnumeratorNameAsString` (`PhysicalMaterial.SurfaceType` _physmat))))
            (:`then`
              (bind (_surface _soundcue _particle _decal) (break `/Game/Blueprints/FBulletEffect` _returnvalue_3))
              (`GameplayStatics.PlaySoundAtLocation` _soundcue _location (struct) 1.0 1.0 0.0 null null null null)
              (`GameplayStatics.SpawnEmitterAttached` _particle _hitcomponent _hitbonename _location (`KismetMathLibrary.MakeRotFromZ` (`KismetMathLibrary.GetReflectionVector` (`KismetMathLibrary.GetDirectionUnitVector` _tracestart _traceend) _impactnormal)) (1.0 1.0 1.0) "KeepWorldPosition" true "AutoRelease")
              (bind _returnvalue_4 (`GameplayStatics.SpawnDecalAttached` _decal (4.0 4.0 4.0) _hitcomponent _hitbonename _location (`self.NewMacro` _normal) "KeepWorldPosition" 3.0))
              (`/Engine/EditorBlueprintResources/StandardMacros.IsValid` _returnvalue_4
                (:`Is Valid`
                  (`DecalComponent.SetFadeScreenSize` _returnvalue_4 1e-05))))))))
    (:`then_2`
      (`self.K2_DestroyActor`))))

(fn `UserConstructionScript`)