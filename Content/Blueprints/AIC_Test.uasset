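; AIC_Test is a test Blueprint, apparently an AI controller, that logs AI Perception events for debugging.
; Perception updates, target info updates and forgotten targets each print a message, with the latter two naming the target and info updates adding its ID.
; OnTargetPerceptionUpdated, BeginPlay, Tick and the construction script are empty, so the asset drives no behavior of its own in these graphs.
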(event `self.AIPerception.OnTargetPerceptionUpdated`
  (params (Actor :type "Actor Object Reference") (Stimulus :type "AIStimulus Structure")))

(event `self.AIPerception.OnTargetPerceptionForgotten`
  (params (Actor :type "Actor Object Reference"))
  (`KismetSystemLibrary.PrintString` (`KismetStringLibrary.Concat_StrStr` " TargetPerceptionFoggot :" (`KismetSystemLibrary.GetDisplayName` Actor))))

(event `self.AIPerception.OnTargetPerceptionInfoUpdated`
  (params (UpdateInfo :type "ActorPerceptionUpdateInfo Structure (by ref)"))
  (bind (_targetid _target) (break `ActorPerceptionUpdateInfo` UpdateInfo))
  (`KismetSystemLibrary.PrintString` (`KismetStringLibrary.Concat_StrStr` " TargetPerceptionInfoUpdate" (`KismetSystemLibrary.GetDisplayName` _target) (`KismetStringLibrary.Conv_IntToString` _targetid))))

(event `self.AIPerception.OnPerceptionUpdated`
  (params (UpdatedActors :type "Array of Actor Object Reference (by ref)"))
  (`KismetSystemLibrary.PrintString` "PerceptionUpdate"))

(fn `UserConstructionScript`)