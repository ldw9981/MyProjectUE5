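; BP_IntervalSpawner is an actor that repeatedly spawns a configurable class at its own transform on a timed interval.
; On BeginPlay, if the class is valid, it starts a looping timer with configurable initial delay and variance, storing the handle.
; Each tick of the timer spawns an actor and records it in an array.
; StopAndClear cancels the timer and destroys every still-valid spawned actor.
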(event `self.ReceiveBeginPlay`
  (`self.Class`
    (:`then`
      (bind _returnvalue (`KismetSystemLibrary.K2_SetTimerDelegate` (delegate `커스텀이벤트_0`) (`self.Interval`) true (`self.Initial Start Delay`) (`self.Initial Start Delay Variance`)))
      (set `self.Timer` _returnvalue))
    (:`else`)))

(event `커스텀이벤트_0`
  (bind _returnvalue (`|SpawnActorFromClass` (`self.Class`) (`self.GetTransform`) "Undefined" "OverrideRootScale" null null))
  (`KismetArrayLibrary.Array_Add` (`self.NewVar`) _returnvalue))

(fn `StopAndClear`
  (`KismetSystemLibrary.K2_ClearAndInvalidateTimerHandle` (`self.Timer`))
  (for _array_element (`self.NewVar`)
    (`/Engine/EditorBlueprintResources/StandardMacros.IsValid` _array_element
      (:`Is Valid`
        (`self.K2_DestroyActor` _array_element)))))

(fn `UserConstructionScript`)