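; BP_PlayerBase is an actor with a health widget that also runs the level's timed clear condition.
; On BeginPlay it initializes WBP_Health with itself, starts a one-shot ClearTime timer and hides the referenced portal (Potal).
; When the timer fires, it calls StopAndClear on every BP_IntervalSpawner and unhides the portal inside that loop, so the reveal requires at least one spawner.
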(event `self.ReceiveBeginPlay`
  (bind _aswbp_health (cast `/Game/Blueprints/Widget/WBP_Health` (`WidgetComponent.GetUserWidgetObject` (`self.Widget`))))
  (`/Game/Blueprints/Widget/WBP_Health.Initialize` _aswbp_health self)
  (`KismetSystemLibrary.K2_SetTimerDelegate` (delegate `커스텀이벤트`) (`self.ClearTime`))
  (bind _potal (`self.Potal`)
    (:`then`
      (`/Game/Blueprints/BP_Portal.Hide` _potal true))
    (:`else`)))

(event `커스텀이벤트`
  (bind _outactors (`GameplayStatics.GetAllActorsOfClass` "/Game/Blueprints/BP_IntervalSpawner.BP_IntervalSpawner_C"))
  (for _array_element _outactors
    (`/Game/Blueprints/BP_IntervalSpawner.StopAndClear` _array_element)
    (bind _potal (`self.Potal`)
      (:`then`
        (`/Game/Blueprints/BP_Portal.Hide` _potal false))
      (:`else`))))

(fn `UserConstructionScript`)