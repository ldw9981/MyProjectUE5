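; BP_Obstacle is a destructible obstacle actor with a health stat and a health widget.
; On BeginPlay it casts its widget component's user widget to WBP_Health and initializes it with itself.
; When the BP_AbilityStat component reports health at or below zero, Death destroys the actor.
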(event `self.ReceiveBeginPlay`
  (bind _aswbp_health (cast `/Game/Blueprints/Widget/WBP_Health` (`WidgetComponent.GetUserWidgetObject` (`self.Widget`))))
  (`/Game/Blueprints/Widget/WBP_Health.Initialize` _aswbp_health self))

(event `self.BP_AbilityStat.OnChangeHealth`
  (params (Prev :type "Float (double-precision)") (Curr :type "Float (double-precision)"))
  (if (<= Curr 0.0)
    (`self.Death`)))

(fn `Death`
  (`self.K2_DestroyActor`))

(fn `UserConstructionScript`)