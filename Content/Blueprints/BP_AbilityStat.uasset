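; BP_AbilityStat is a component that holds Health, Defense and Attack stats for its owning actor.
; On BeginPlay it copies the initial values and binds to the owner's OnTakeAnyDamage, reducing incoming damage by Defense while Health is above zero.
; All health changes go through SetHealth, which broadcasts OnChangeHealth with previous and current values.
; AddHealth heals up to InitialMaxHealth, and GetHealthPercent returns the ratio to that maximum.
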(event `self.ReceiveBeginPlay`
  (add `Actor.OnTakeAnyDamage` (`self.GetOwner`) (delegate `OnTakeAnyDamage_이벤트`))
  (set `self.Health` (`self.InitialMaxHealth`))
  (set `self.Defense` (`self.InitialDefense`))
  (set `self.Attack` (`self.InitialAttack`)))

(event `OnTakeAnyDamage_이벤트`
  (params (DamagedActor :type "Actor Object Reference") (Damage :type "Float (single-precision)") (DamageType :type "DamageType Object Reference") (InstigatedBy :type "Controller Object Reference") (DamageCauser :type "Actor Object Reference"))
  ;[1 1 1] 살아있을때만 처리
  (if (> (`self.Health`) 0.0)
    (`self.SetHealth` (`KismetMathLibrary.FMax` (- (`self.Health`) (`KismetMathLibrary.FMax` (- Damage (`self.Defense`))))))))

(fn `AddHealth`
  (params (value :type "Float (double-precision)"))
  (`self.SetHealth` (`KismetMathLibrary.FMin` (+ (`self.Health`) value) (`self.InitialMaxHealth`))))

(fn `GetHealthPercent`
  (returns (Percent :type "Float (double-precision)"))
  (return (/ (`self.Health`) (`self.InitialMaxHealth`))))

(fn `SetHealth`
  (params (Value :type "Float (double-precision)"))
  (locals (Prev :type "Float (double-precision)"))
  (set `local.Prev` (`self.Health`))
  (set `self.Health` Value)
  (`self.OnChangeHealth` (`local.Prev`) (`self.Health`)))