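; BP_MovingFlatform is a moving platform that loops its StaticMesh along a path defined by a vector Curve.
; Each tick, game time plus a Variation offset wraps by the curve's maximum time and samples the mesh's relative location.
; The construction script applies the same function with Variation alone, placing the mesh at its phase-offset starting point.
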(event `self.ReceiveBeginPlay`)

(event `self.ReceiveTick`
  (params (DeltaSeconds :type "Float (single-precision)"))
  (`self.UpdateRelativeLocation` (+ (`self.Variation`) (`KismetSystemLibrary.GetGameTimeInSeconds`))))

(fn `UpdateRelativeLocation`
  (params (A :type "Float (double-precision)"))
  (`SceneComponent.K2_SetRelativeLocation` (`self.StaticMesh`) (`CurveVector.GetVectorValue` (`self.Curve`) (mod A (`.MaxTime` (`CurveBase.GetTimeRange` (`self.Curve`))))) false false))

(fn `UserConstructionScript`
  (`self.UpdateRelativeLocation` (`self.Variation`)))