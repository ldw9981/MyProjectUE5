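; AIC_Monster is a monster AI controller that turns sight and damage perception into Blackboard targets.
; Sighting the player character sets the Player key, and losing sight starts a short grace timer that clears it unless the player is seen again.
; Damage stimuli treat the sensed actor as a Controller and store its pawn as Attacker, clearing that key when the stimulus is not successfully sensed.
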(event `self.AIPerception.OnTargetPerceptionUpdated`
  (params (Actor :type "Actor Object Reference") (Stimulus :type "AIStimulus Structure"))
  (bind _blackboard (`self.Blackboard`))
  (bind _returnvalue (`AIPerceptionSystem.GetSenseClassForStimulus` Stimulus))
  (if (== _returnvalue "/Script/AIModule.AISense_Sight")
    (if (== Actor (`GameplayStatics.GetPlayerCharacter` 0))
      ;[1 1 1] true 시야에있음,false 시야에서 나감
      (if (`.bSuccessfullySensed` (break `AIStimulus` Stimulus))
        (`KismetSystemLibrary.K2_ClearAndInvalidateTimerHandle` (`self.TimerPlayerNull`))
        (`BlackboardComponent.SetValueAsObject` (`self.Blackboard`) "Player" Actor)
        (else
          (bind _returnvalue_2 (`KismetSystemLibrary.K2_SetTimerDelegate` (delegate `커스텀이벤트`) 3.0))
          (set `self.TimerPlayerNull` _returnvalue_2))))
    (elif (== _returnvalue "/Script/AIModule.AISense_Damage")
      (if (`.bSuccessfullySensed` (break `AIStimulus` Stimulus))
        (bind `_as컨트롤러` (cast `Controller` Actor))
        (`BlackboardComponent.SetValueAsObject` _blackboard "Attacker" (`self.K2_GetPawn` `_as컨트롤러`))
        (else
          (`BlackboardComponent.SetValueAsObject` _blackboard "Attacker" null))))))

(event `커스텀이벤트`
  ;[1 1 1] true 시야에있음,false 시야에서 나감
  (`BlackboardComponent.SetValueAsObject` (`self.Blackboard`) "Player" null))

(fn `UserConstructionScript`)