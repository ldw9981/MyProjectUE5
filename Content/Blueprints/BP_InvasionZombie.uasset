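; Invasion zombie enemy that runs BT_InvasionMonster, seeding its blackboard with the player base and health percent.
; BPAbilityStat feeds the health widget and updates that percent; at zero health it grants DT_MonsterInfo rewards, disables collision and AI, then destroys itself after a delay.
; Helper events damage the blackboard's AITarget and knock the zombie away from radial damage causers.
; Stat initialization from the data table in the construction script is disconnected.
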(event `self.ReceiveBeginPlay`
  (bind _returnvalue (`AIBlueprintHelperLibrary.GetAIController` self))
  (bind _blackboard (`AIController.Blackboard` _returnvalue))
  (`|ExecutionSequence`
    (:`then_0`
      (bind _aswbp_health (cast `/Game/Blueprints/Widget/WBP_Health` (`WidgetComponent.GetUserWidgetObject` (`self.Widget`))))
      (set `/Game/Blueprints/Widget/WBP_Health.AbilityStat` (`self.BP_AbilityStat`) _aswbp_health)
      (set `/Game/Blueprints/Widget/WBP_Health.OwnerActor` self _aswbp_health))
    (:`then_1`
      (bind _returnvalue_2 (`AIController.RunBehaviorTree` _returnvalue "/Game/Blueprints/AI/BT_InvasionMonster.BT_InvasionMonster"))
      (if _returnvalue_2
        ;[1 1 1] 초기 HealthPercent 1.0을 블랙보드에 기록
        (bind _percent (`/Game/Blueprints/BP_AbilityStat.GetHealthPercent` (`self.BP_AbilityStat`)))
        (`BlackboardComponent.SetValueAsFloat` _blackboard "HealthPercent" _percent)
        (bind _returnvalue_3 (`GameplayStatics.GetActorOfClass` "/Game/Blueprints/BP_PlayerBase.BP_PlayerBase_C"))
        (`BlackboardComponent.SetValueAsObject` _blackboard "PlayerBase" _returnvalue_3)))))

(event `self.ReceiveActorBeginOverlap`
  (params (OtherActor :type "Actor Object Reference")))

(event `self.BP_AbilityStat.OnChangeHealth`
  (params (Prev :type "Float (double-precision)") (Curr :type "Float (double-precision)"))
  (if (<= Curr 0.0)
    (`|ExecutionSequence`
      (:`then_0`
        (bind _asbp_my_player_character (cast `/Game/Blueprints/BP_MyPlayerCharacter` (`GameplayStatics.GetPlayerCharacter` 0)))
        (bind _returnvalue (`|GetDataTableRow` "/Game/Blueprints/Data/DT_MonsterInfo.DT_MonsterInfo" (`self.MonsterID`))
          (:`then`
            (bind (_name _level _health _attack _defense _rewardgold _rewardexp _rewardscore) (break `/Game/Blueprints/FMonsterInfo` _returnvalue))
            (`/Game/Blueprints/BP_MyPlayerCharacter.GetReward` _asbp_my_player_character _rewardexp _rewardgold _rewardscore))))
      (:`then_1`
        (`PrimitiveComponent.SetCollisionEnabled` (`self.CapsuleComponent`) "NoCollision")
        (`BrainComponent.StopLogic` (`AIController.BrainComponent` (`AIBlueprintHelperLibrary.GetAIController` self)) ""))
      (:`then_2`
        (`KismetSystemLibrary.Delay` 3.0)
        (`self.K2_DestroyActor`)))
    (else
      ;[1 1 1] 현재 HealthPercent를 블랙보드에 기록
      (bind _percent (`/Game/Blueprints/BP_AbilityStat.GetHealthPercent` (`self.BP_AbilityStat`)))
      (`BlackboardComponent.SetValueAsFloat` (`AIController.Blackboard` (`AIBlueprintHelperLibrary.GetAIController` self)) "HealthPercent" _percent))))

(event `/Game/Blueprints/BPI_AnimNotify.ApplyDamageAITarget`
  (params (BaseDamage :type "Float (double-precision)"))
  (bind `_as액터` (cast `Actor` (`BlackboardComponent.GetValueAsObject` (`AIBlueprintHelperLibrary.GetBlackboard` null) "AITarget")))
  (`GameplayStatics.ApplyDamage` `_as액터` BaseDamage))

(event `self.ReceiveRadialDamage`
  (params (DamageReceived :type "Float (single-precision)") (DamageType :type "DamageType Object Reference") (Origin :type "Vector Structure") (HitInfo :type "HitResult Structure (by ref)") (InstigatedBy :type "Controller Object Reference") (DamageCauser :type "Actor Object Reference"))
  ;[1 1 1] 좀비 속도0 변경
  (`MovementComponent.StopMovementImmediately` (`self.CharacterMovement`))
  (`CharacterMovementComponent.AddImpulse` (`self.CharacterMovement`) (* (`KismetMathLibrary.GetDirectionUnitVector` (`self.K2_GetActorLocation` DamageCauser) (`self.K2_GetActorLocation`)) 100000.0) false))

(fn `UserConstructionScript`
  ;[1 1 1] 블루프린트를 수정하거나 게임을 시작할때 BeginPlay이전에 호출함
)