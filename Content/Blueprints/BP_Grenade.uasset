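; BP_Grenade is a thrown or launched grenade projectile that explodes on a fixed fuse after spawning.
; The construction script copies initial and max speed variables into its ProjectileMovement component.
; BeginPlay starts a one-shot timer whose custom event spawns an explosion emitter, applies radial damage credited to the instigator controller, then destroys the actor.
; The blast also draws a debug sphere at the damage radius; overlaps do not trigger it.
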(event `self.ReceiveBeginPlay`
  (`KismetSystemLibrary.K2_SetTimerDelegate` (delegate `커스텀이벤트`) 3.0))

(event `커스텀이벤트`
  (bind _returnvalue (`self.K2_GetActorLocation`))
  (bind _damage_radius (`self.Damage Radius`))
  (`GameplayStatics.SpawnEmitterAtLocation` "/Game/StarterContent/Particles/P_Explosion.P_Explosion" (`self.K2_GetActorLocation`) (struct) (3.0 3.0 3.0))
  (`GameplayStatics.ApplyRadialDamage` :`BaseDamage` (`self.Base Damage`) :`Origin` _returnvalue :`DamageRadius` _damage_radius :`DamageCauser` self :`InstigatedByController` (`self.GetInstigatorController`))
  (`KismetSystemLibrary.DrawDebugSphere` _returnvalue _damage_radius 12 (struct :`R` 1.0 :`G` 1.0 :`B` 1.0 :`A` 1.0) 3.0)
  (`self.K2_DestroyActor`))

(fn `UserConstructionScript`
  (bind _projectilemovement (`self.ProjectileMovement`))
  (set `ProjectileMovementComponent.InitialSpeed` (`self.초기 속도`) _projectilemovement)
  (set `ProjectileMovementComponent.MaxSpeed` (`self.최대 속도`) _projectilemovement))